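; Flame pillar actor that makes its fire light flicker continuously from BeginPlay.
; Two timelines supply flame intensity curves, which AdjustIntensity multiplies by BaseIntensity and applies to FireLight.
; Each timeline calls ChooseTimeline on finishing to loop the effect through a random switch.
; Because RandomInteger has a Max of 1, the switch always gets 0, so only the first timeline plays.
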(event `self.ReceiveBeginPlay`
  (`self.ChooseTimeline`))

(event `ChooseTimeline`
  (switch `int` (`KismetMathLibrary.RandomInteger` 1)
    (:`Default`
      (`self.PlayTimeline2` :!label _label))
    (:`0`
      (`self.PlayTimeline1`))
    (:`1`
      (goto _label))))

(event `PlayTimeline1`
  (bind (_direction _flameintensity) (`Timeline|LightIntensity_1` :!via `PlayFromStart`)
    (:`Update`
      (`self.AdjustIntensity` _flameintensity))
    (:`Finished`
      (`self.ChooseTimeline`))))

(event `PlayTimeline2`
  (bind (_direction _flameintensity) (`Timeline|LightIntensity_2` :!via `PlayFromStart`)
    (:`Update`
      (`self.AdjustIntensity` _flameintensity))
    (:`Finished`
      (`self.ChooseTimeline`))))

(fn `AdjustIntensity`
  (params (Intensity :type "Float (double-precision)"))
  (`LightComponent.SetIntensity` (`self.FireLight`) (* Intensity (`self.BaseIntensity`))))

(fn `UserConstructionScript`)