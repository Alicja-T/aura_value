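; Enemy gameplay ability for a ranged attack that fires a projectile at the avatar's combat target.
; On activation it turns the avatar toward the target and plays a random attack montage from those the avatar supplies.
; The montage's tagged gameplay event triggers the projectile toward the target's re-read location, then ends the ability.
; The montage keeps playing after the ability ends, and completion, interruption or cancellation also ends it.
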(event `self.K2_ActivateAbility`
  (bind _returnvalue (`self.GetAvatarActorFromActorInfo`))
  (bind _returnvalue_2 (`self.GetAvatarActorFromActorInfo`))
  (bind (_montage _montagetag) (break `TaggedMontage` (`self.ChosenMontage`)))
  (bind _returnvalue_3 (message `EnemyInterface.GetCombatTarget` _returnvalue))
  (message `CombatInterface.SetFacingTarget` _returnvalue (`Actor.K2_GetActorLocation` _returnvalue_3))
  (bind _returnvalue_4 (message `CombatInterface.GetAttackMontages` _returnvalue))
  (bind _output_get (set `self.ChosenMontage` (`KismetArrayLibrary.Array_Random` _returnvalue_4)))
  (`AbilityTask_PlayMontageAndWait.CreatePlayMontageAndWaitProxy` "None" (`.Montage` (break `TaggedMontage` _output_get)) 1.0 "None" false
    (:`then`
      (`AbilityAsync_WaitGameplayEvent.WaitGameplayEventToActor` _returnvalue_2 _montagetag
        (:`then`
          (message `CombatInterface.GetCombatSocketLocation` _returnvalue_2 _montagetag)
          (bind _returnvalue_5 (message `EnemyInterface.GetCombatTarget` (`self.GetAvatarActorFromActorInfo`)))
          (`self.SpawnProjectile` (`Actor.K2_GetActorLocation` _returnvalue_5))
          (`self.K2_EndAbility`))))
    (:`OnCompleted`
      (`self.K2_EndAbility` :!label _label))
    (:`OnInterrupted`
      (goto _label))
    (:`OnCancelled`
      (goto _label))))