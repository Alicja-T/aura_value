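; Gameplay ability for enemy melee attacks that turns the avatar toward its combat target and plays a random attack montage.
; On the montage's gameplay event, it gathers live players around the matching combat socket and damages any non-friends.
; Each victim spawns its own blood effect, and a hit plays the montage's impact sound once.
; The ability ends after that event or when the montage completes or is interrupted.
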(event `self.K2_ActivateAbility`
  (bind _returnvalue (`self.GetAvatarActorFromActorInfo`))
  (bind _returnvalue_2 (`self.GetAvatarActorFromActorInfo`))
  (set `self.HasHitTarget` false)
  (bind _returnvalue_3 (message `EnemyInterface.GetCombatTarget` _returnvalue))
  (bind _ascombat_interface (cast `CombatInterface` _returnvalue))
  (`CombatInterface.SetFacingTarget` _ascombat_interface (`Actor.K2_GetActorLocation` _returnvalue_3))
  (bind _returnvalue_4 (message `CombatInterface.GetAttackMontages` _returnvalue))
  (bind _output_get (set `self.ChosenMontage` (`KismetArrayLibrary.Array_Random` _returnvalue_4)))
  (bind (_montage _montagetag _impactsound) (break `TaggedMontage` _output_get))
  (`AbilityTask_PlayMontageAndWait.CreatePlayMontageAndWaitProxy` "None" _montage 1.0 "None" false
    (:`then`
      (`AbilityAsync_WaitGameplayEvent.WaitGameplayEventToActor` _returnvalue_2 _montagetag
        (:`EventReceived`
          (bind _returnvalue_5 (message `CombatInterface.GetCombatSocketLocation` _returnvalue_2 _montagetag))
          (bind _outoverlappingactors (`ValueAbilitySystemLibrary.GetLivePlayersWithinRadius` _returnvalue_2 (`|MakeArray` _returnvalue_2) 100.0 _returnvalue_5))
          (for _array_element _outoverlappingactors
            (if (`ValueAbilitySystemLibrary.IsNotFriend` _array_element (`self.GetAvatarActorFromActorInfo`))
              (`self.CauseDamage` _array_element)
              (set `self.HasHitTarget` true)
              (bind _returnvalue_6 (message `CombatInterface.GetBloodEffect` _array_element))
              (`NiagaraFunctionLibrary.SpawnSystemAtLocation` _returnvalue_6 _returnvalue_5)))
          (if (`self.HasHitTarget`)
            (`GameplayStatics.PlaySoundAtLocation` _impactsound _returnvalue_5 (struct) 1.0 1.0 0.0 null null null null))
          (`self.K2_EndAbility`))))
    (:`OnCompleted`
      (`self.K2_EndAbility` :!label _label))
    (:`OnInterrupted`
      (goto _label))
    (:`OnCancelled`
      (goto _label))))