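; Enemy gameplay ability that summons random minions around the caster's computed spawn locations.
; On activation it gets and shuffles the spawn locations, then plays a Niagara ground summon effect at each.
; After a short delay, an index-driven Delay loop spawns minions one at a time slightly above those points, each with its default controller.
; The graph never calls EndAbility.
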(event `self.K2_ActivateAbility`
  (bind _returnvalue (`self.GetSpawnLocations`))
  (bind _output_get (set `self.SpawnLocations` _returnvalue))
  (`KismetArrayLibrary.Array_Shuffle` _output_get)
  (for _array_element (`self.SpawnLocations`)
    (`NiagaraFunctionLibrary.SpawnSystemAtLocation` "/Game/Assets/Effects/Combat/NS_GroundSummon.NS_GroundSummon" _array_element)
    (`KismetSystemLibrary.Delay` 1.5)
    (if (< (`self.SpawnIndex`) (`KismetArrayLibrary.Array_Length` (`self.SpawnLocations`))) :!label _label
      (bind _returnvalue_2 (`|SpawnActorFromClass` (`self.GetRandomMinionClass`) (`KismetMathLibrary.MakeTransform` (+ (`|GetArrayItem` (`self.SpawnLocations`) (`self.SpawnIndex`)) (0.0 0.0 100.0))) "AlwaysSpawn" "MultiplyWithRoot" null null))
      (`Pawn.SpawnDefaultController` _returnvalue_2)
      (bind _result (`/Engine/EditorBlueprintResources/StandardMacros.IncrementInt` (`self.SpawnIndex`))
        (:`  `
          (set `self.SpawnIndex` _result)
          (`KismetSystemLibrary.Delay` 3.0)
          (goto _label))))))