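; Firebolt gameplay ability that casts a projectile at the location under the mouse.
; On activation it gets target data under the mouse, turns the avatar toward the hit location through CombatInterface and plays the cast montage.
; While the montage plays, it waits for the Firebolt montage gameplay event and spawns the projectile toward the target when received.
; EndAbility is present but unconnected, so this graph never ends the ability.
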(event `self.K2_ActivateAbility`
  (bind (_asynctaskproxy _datahandle) (`TargetDataUnderMouse.CreateTargetDataUnderMouse`)
    (:`ValidData`
      (set `self.TargetLocation` (`.Location` (`GameplayStatics.BreakHitResult` (`AbilitySystemBlueprintLibrary.GetHitResultFromTargetData` _datahandle))))
      (bind _ascombat_interface (cast `CombatInterface` (`self.GetAvatarActorFromActorInfo`)))
      (`CombatInterface.SetFacingTarget` _ascombat_interface (`self.TargetLocation`))
      (`AbilityTask_PlayMontageAndWait.CreatePlayMontageAndWaitProxy` "None" "/Game/Assets/Characters/Aura/Animations/Abilities/AM_CastFirebolt.AM_CastFirebolt"
        (:`then`
          (`AbilityTask_WaitGameplayEvent.WaitGameplayEvent` (struct :`TagName` "Event.Montage.Firebolt") null
            (:`EventReceived`
              (`self.SpawnProjectile` (`self.TargetLocation`)))))))))